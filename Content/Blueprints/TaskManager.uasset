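; Task manager for the MR pawn's tasks, such as the shopping task, loading definitions from a JSON file in the content directory.
; CreateTask constructs a Task object from its class name and initializes it with a spawned grasping object as evaluation point.
; While Evaluation is on, Tick evaluates the task until finished and triggers the pawn's StartButtonClicked when no items remain.
; InitializeTaskInterface makes the evaluation point immovable and returns shopping-list text for shopping tasks.
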(event EventBeginPlay
  (Variables|Default|SetEvaluation false))

(event EventTick
  (params (DeltaSeconds :type Float%20%28single-precision%29))
  (bind _task (Variables|Default|GetTask))
  (if (Variables|Default|GetEvaluation)
    (Class|Task|Evaluate _task)
    (Variables|Default|SetEvaluation (not (Class|Task|IsTaskFinished _task)))
    (if (== (Utilities|Array|Length (Class|Task|GetTaskItems _task (Utilities|Array|MakeArray))) 0)
      (bind _asmrpawn (Utilities|Casting|CastToMRPawn (Game|Player|GetPlayerPawn 0)))
      (Default|StartButtonClicked _asmrpawn))))

(fn ConstructionScript)

(fn LoadTasks
  (params (Filename :type String))
  (bind _returnvalue (Class|Task|LoadTasksfromJSON (Utilities|String|Append (Class|KismetSystemLibrary|GetProjectContentDirectory) Filename)))
  (Variables|Default|SetTasks _returnvalue))

(fn CreateTask
  (params (TaskId :type String))
  (bind _tasks (Variables|Default|GetTasks))
  (bind (_value _returnvalue) (Utilities|Map|Find _tasks TaskId))
  (bind _classname (Utilities|Struct|BreakTaskInfo _value))
  (bind _returnvalue_2 (Class|Task|GetTaskClassbyName _classname))
  (Development|PrintString (Utilities|GetClassDisplayName _returnvalue_2))
  (if _returnvalue
    (bind _returnvalue_3 (Game|ConstructObjectfromClass _returnvalue_2 self))
    (bind _astask (Utilities|Casting|CastToTask _returnvalue_3))
    (bind _output_get (Variables|Default|SetTask _astask))
    (bind _returnvalue_4 (Class|GraspingObject|SpawnGraspingObject "0, 0, 0" "0, 0, 0" "0, 0, 0" (Variables|/Script/HoloDemtect.Task|Geteval_point_info _output_get))) ; TODO: pos, size and rot
    (Class|Task|Initialize _output_get _returnvalue_4 _value))
  (return _returnvalue))

(fn InitializeTaskInterface
  (bind _task (Variables|Default|GetTask))
  (Variables|/Script/HoloDemtect.GraspingObject|Setmovable (Variables|/Script/HoloDemtect.Task|Getevaluation_point _task) false)
  (return (select (== (Utilities|GetClass _task) "/Script/HoloDemtect.ShoppingTask") (Utilities|String|Append "Shopping List: 
" (Utilities|String|JoinStringArray (Class|Task|GetTaskItems _task (Utilities|Array|MakeArray)) " 
")) "")))