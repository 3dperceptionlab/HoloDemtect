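; Mixed reality pawn that drives a task evaluation session from language selection to task end.
; It chains event-bound screens on spawned widget actors: language, setup, task menu from JSON, and ready prompt.
; TaskManager creates the task and validates objects spawned by QRTracking before evaluation, with hand-menu buttons confirming setup and ending the task.
; A separate event shows a data-sending screen, refreshed by timer from the dataset's timeseries length.
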(event Custom|Button1HandMenuClicked
  (bind _qrtracking (Variables|Default|GetQRTracking))
  (bind _taskmanager (Variables|Default|GetTaskManager))
  (bind _task (Variables|/Game/Blueprints/TaskManager.TaskManager_C|GetTask _taskmanager))
  (bind _qritemdict (Variables|/Game/Blueprints/QRTracking.QRTracking_C|GetQRItemDict _qrtracking))
  (bind _spawned_objects (Variables|/Script/HoloDemtect.QRItemDictionary|Getspawned_objects _qritemdict))
  ;[1 1 1] Setup environment (QR codes -> spawn grasping objects and task preparation)
  (if (Class|Task|AreObjectsValid _task _spawned_objects)
    (Variables|Default|SetSpawnedObjects _spawned_objects)
    (Actor|DestroyActor (stale Custom|TaskSelectedMenu _returnvalue_3))
    (Actor|DestroyActor (stale Custom|TaskSelectedMenu _returnvalue_2))
    ;[1 1 1] Ready for user
    (bind _returnvalue (Game|SpawnActorfromClass "/Game/Blueprints/WidgetIntroActor.WidgetIntroActor_C" (Math|Transform|MakeTransform "0, 0, 0") "Undefined" self 0))
    (bind _returnvalue_2 (UserInterface|CreateWidget "/Game/Blueprints/WidgetReadyBlueprint.WidgetReadyBlueprint_C"))
    (UserInterface|SetWidget (Variables|/Game/Blueprints/WidgetIntroActor.WidgetIntroActor_C|GetWidget _returnvalue) _returnvalue_2)
    (bind _aswidget_ready_blueprint (Utilities|Casting|CastToWidgetReadyBlueprint (UserInterface|GetWidget (Variables|/Game/Blueprints/WidgetIntroActor.WidgetIntroActor_C|GetWidget _returnvalue))))
    (EventDispatchers|BindEventtoReadyButtonClicked _aswidget_ready_blueprint (delegate Custom|ReadyButtonClicked))
    (else
      (Development|PrintString "NOT VALID" true true "(R=0.000000,G=0.660000,B=1.000000,A=1.000000)" 1e+01)
      (bind _names (Default|ItemIDArraytoNames (Variables|Default|GetTaskManager) (Class|Task|GetTaskItems _task _spawned_objects)))
      (Default|CallHandMenuText (Utilities|String|Append (Utilities|String|ToString(Text) (Utilities|Text|MakeLiteralText "Objects needed: 
")) (Utilities|String|JoinStringArray _names " 
"))))))

(event Custom|StartButtonClicked
  (bind _returnvalue (Math|Transform|MakeTransform "0, 0, 0"))
  (bind _self self)
  (Actor|DestroyActor (stale EventBeginPlay _returnvalue))
  ;[1 1 1] Task selection and instanciation
  (bind _returnvalue_2 (Game|SpawnActorfromClass "/Game/Blueprints/TaskManager.TaskManager_C" _returnvalue "Undefined" _self 0))
  (bind _output_get (Variables|Default|SetTaskManager _returnvalue_2))
  (Default|LoadTasks _output_get "JSONDicts/tasks.json")
  (bind _returnvalue_3 (Game|SpawnActorfromClass "/Game/Blueprints/WidgetIntroActor.WidgetIntroActor_C" _returnvalue "Undefined" _self 0))
  (bind _returnvalue_4 (UserInterface|CreateWidget "/Game/Blueprints/TaskMenuBP.TaskMenuBP_C"))
  (UserInterface|SetWidget (Variables|/Game/Blueprints/WidgetIntroActor.WidgetIntroActor_C|GetWidget _returnvalue_3) _returnvalue_4)
  (bind _astask_menu (Utilities|Casting|CastToTaskMenu (UserInterface|GetWidget (Variables|/Game/Blueprints/WidgetIntroActor.WidgetIntroActor_C|GetWidget _returnvalue_3)))
    (:then
      (Class|TaskMenu|SetTasks _astask_menu (Variables|/Game/Blueprints/TaskManager.TaskManager_C|GetTasks (Variables|Default|GetTaskManager)))
      (EventDispatchers|BindEventtoOnButtonClickedEvent _astask_menu (delegate Custom|TaskSelectedMenu)))
    (:CastFailed
      (Development|PrintString "Error casting to TaskMenu" true true "(R=1.000000,G=0.029525,B=0.000000,A=1.000000)"))))

(event Custom|ReadyButtonClicked
  ;[1 1 1] Ready for user
  (Actor|DestroyActor (stale Custom|Button1HandMenuClicked _returnvalue))
  (bind _returnvalue (Game|SpawnActorfromClass "/Game/Blueprints/WidgetHandMenu.WidgetHandMenu_C" (Math|Transform|MakeTransform "0, 0, 0") "Undefined" self 0))
  (EventDispatchers|BindEventtoButton1HandMenuClicked _returnvalue (delegate Custom|ButtonHandDuringTask))
  (bind _tasklisttext (Default|StartEvaluation (Variables|Default|GetTaskManager)))
  (Default|CallHandMenuText _tasklisttext)
  (bind _asuxt_pressable_button_actor (Utilities|Casting|CastToUxtPressableButtonActor (Variables|/Script/Engine.ChildActorComponent|GetChildActor (Variables|/UXToolsExamples/HandMenu/Blueprints/BP_SmallHandMenu.BP_SmallHandMenu_C|GetButton_2 _returnvalue)))
    (:then
      (Rendering|Components|TextRender|SetText (Variables|/Script/UXTools.UxtPressableButtonActor|GetLabelComponent _asuxt_pressable_button_actor) (Utilities|Text|MakeLiteralText "Finish task"))
      (Rendering|Components|TextRender|SetText (Variables|/Script/UXTools.UxtPressableButtonActor|GetIconComponent _asuxt_pressable_button_actor) (Utilities|Text|MakeLiteralText "E894")))
    (:CastFailed
      (Development|PrintString "Cast to UxtPressableButton FAIL" true true "(R=1.000000,G=0.000000,B=0.025124,A=1.000000)"))))

(event Custom|ButtonHandDuringTask
  ;[1 1 1] Ready for user
  (Default|EndTask (Variables|Default|GetTaskManager)))

(event Custom|TaskSelectedMenu
  (params (button :type String))
  (bind _returnvalue (Math|Transform|MakeTransform "0, 0, 0"))
  (bind _self self)
  ;[1 1 1] Task selection and instanciation
  (bind _output (Default|CreateTask (Variables|Default|GetTaskManager) button))
  (if _output
    (Actor|DestroyActor (stale Custom|StartButtonClicked _returnvalue_3))
    ;[1 1 1] Setup environment (QR codes -> spawn grasping objects and task preparation)
    (bind _returnvalue_2 (Game|SpawnActorfromClass "/Game/Blueprints/QRTracking.QRTracking_C" _returnvalue "Undefined" _self 0))
    (Variables|Default|SetQRTracking _returnvalue_2)
    (bind _returnvalue_3 (Game|SpawnActorfromClass "/Game/Blueprints/WidgetHandMenu.WidgetHandMenu_C" _returnvalue "Undefined" _self 0))
    (EventDispatchers|BindEventtoButton1HandMenuClicked _returnvalue_3 (delegate Custom|Button1HandMenuClicked))
    (bind _names (Default|ItemIDArraytoNames (Variables|Default|GetTaskManager) (Class|Task|GetTaskItems (Variables|/Game/Blueprints/TaskManager.TaskManager_C|GetTask (Variables|Default|GetTaskManager)) (Variables|/Script/HoloDemtect.QRItemDictionary|Getspawned_objects (Variables|/Game/Blueprints/QRTracking.QRTracking_C|GetQRItemDict (Variables|Default|GetQRTracking))))))
    (Default|CallHandMenuText (Utilities|String|Append (Utilities|String|ToString(Text) (Utilities|Text|MakeLiteralText "Objects needed: 
")) (Utilities|String|JoinStringArray _names " 
")))
    (else
      (EventDispatchers|BindEventtoOnButtonClickedEvent (stale Custom|StartButtonClicked _astask_menu) (delegate Custom|TaskSelectedMenu)))))

(event Custom|WaitingWhileSendingData
  ;[1 1 1] Ready for user
  (bind _returnvalue (Game|SpawnActorfromClass "/Game/Blueprints/WidgetIntroActor.WidgetIntroActor_C" (Math|Transform|MakeTransform "0, 0, 0") "Undefined" self 0))
  (bind _returnvalue_2 (UserInterface|CreateWidget "/Game/Blueprints/WidgetSendindDataBlueprint.WidgetSendindDataBlueprint_C"))
  (UserInterface|SetWidget (Variables|/Game/Blueprints/WidgetIntroActor.WidgetIntroActor_C|GetWidget _returnvalue) _returnvalue_2)
  (bind _aswidget_sendind_data_blueprint (Utilities|Casting|CastToWidgetSendindDataBlueprint (UserInterface|GetWidget (Variables|/Game/Blueprints/WidgetIntroActor.WidgetIntroActor_C|GetWidget _returnvalue))))
  (Utilities|Time|SetTimerbyEvent (delegate Custom|UpdateSendingDataUI) 1.0 true))

(event Custom|UpdateSendingDataUI
  ;[1 1 1] Ready for user
  (Default|UpdateInfo (stale Custom|WaitingWhileSendingData _aswidget_sendind_data_blueprint) (Utilities|Array|Length (Variables|/Script/HoloDemtect.DatasetGenerator|Gettimeseries (Variables|/Game/Blueprints/TaskManager.TaskManager_C|GetDatasetGenerator (Variables|Default|GetTaskManager))))))

(event Custom|Language%20Selected
  (params (Language :type String))
  ;[1 1 1] Intro text
  (Class|KismetInternationalizationLibrary|SetCurrentCulture Language)
  (Utilities|FlowControl|Delay 0.2)
  (bind _returnvalue (UserInterface|CreateWidget "/Game/Blueprints/WidgetSetupBlueprint.WidgetSetupBlueprint_C"))
  (UserInterface|SetWidget (Variables|/Game/Blueprints/WidgetIntroActor.WidgetIntroActor_C|GetWidget (stale EventBeginPlay _returnvalue)) _returnvalue)
  (bind _aswidget_setup_blueprint (Utilities|Casting|CastToWidgetSetupBlueprint (UserInterface|GetWidget (Variables|/Game/Blueprints/WidgetIntroActor.WidgetIntroActor_C|GetWidget (stale EventBeginPlay _returnvalue)))))
  (EventDispatchers|BindEventtoStartButtonClicked _aswidget_setup_blueprint (delegate Custom|StartButtonClicked)))

(event EventBeginPlay
  (bind _returnvalue (Game|SpawnActorfromClass "/Game/Blueprints/WidgetIntroActor.WidgetIntroActor_C" (Math|Transform|MakeTransform "0, 0, 0") "Undefined" self 0))
  (bind _returnvalue_2 (UserInterface|CreateWidget "/Game/Blueprints/WidgetLangBlueprint.WidgetLangBlueprint_C"))
  (UserInterface|SetWidget (Variables|/Game/Blueprints/WidgetIntroActor.WidgetIntroActor_C|GetWidget _returnvalue) _returnvalue_2)
  (bind _aswidget_lang_blueprint (Utilities|Casting|CastToWidgetLangBlueprint (UserInterface|GetWidget (Variables|/Game/Blueprints/WidgetIntroActor.WidgetIntroActor_C|GetWidget _returnvalue)))
    (:then
      (EventDispatchers|BindEventtoLanSelected _aswidget_lang_blueprint (delegate Custom|Language%20Selected)))
    (:CastFailed
      (Development|PrintString "Error casting to WidgetLang" true true "(R=1.000000,G=0.029525,B=0.000000,A=1.000000)"))))

(fn ConstructionScript)