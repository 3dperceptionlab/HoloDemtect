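; Tracks AR QR codes and spawns the items mapped to them in a JSON dictionary loaded from qr_objects.json.
; QR capture starts on a short timer after BeginPlay and stops at EndPlay.
; Tracked-geometry updates skip codes near the X/Y origin, then spawn each known code once, using a boolean semaphore and a spawned list.
; Colored debug boxes mark spawned, known and unknown codes.
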(event OnUpdateTrackedGeometry(ARTrackableNotify)
  (params (TrackedGeometry :type AR%20Tracked%20Geometry%20Object%20Reference))
  (bind _spawedqrs (Variables|Default|GetSpawedQRs))
  (bind _qritemdict (Variables|Default|GetQRItemDict))
  (bind _asartracked_qrcode (Utilities|Casting|CastToARTrackedQRCode TrackedGeometry))
  (Development|PrintString "CROQUETAS!!!!!!!" false false)
  (if (Utilities|IsValid _asartracked_qrcode)
    (if (Math|Boolean|NANDBoolean (< (Math|Float|Absolute(Float) (.x (.location (Class|ARTrackedGeometry|GetLocaltoWorldTransform _asartracked_qrcode)))) 0.01) (< (Math|Float|Absolute(Float) (.y (.location (Class|ARTrackedGeometry|GetLocaltoWorldTransform _asartracked_qrcode)))) 0.01)) ; Location ok
      (if (Utilities|Set|Contains _spawedqrs (Variables|/Script/AugmentedReality.ARTrackedQRCode|GetQRCode _asartracked_qrcode)) ; Spawned
        (Rendering|Debug|DrawDebugBox (Math|Transform|TransformLocation (Class|ARTrackedGeometry|GetLocaltoWorldTransform _asartracked_qrcode) (/ (Math|Vector|MakeVector 0.3 (.X (Math|Vector2D|BreakVector2D (Class|ARTrackedImage|GetEstimateSize _asartracked_qrcode))) (.Y (Math|Vector2D|BreakVector2D (Class|ARTrackedImage|GetEstimateSize _asartracked_qrcode)))) 2.0)) (/ (Math|Vector|MakeVector 0.3 (.X (Math|Vector2D|BreakVector2D (Class|ARTrackedImage|GetEstimateSize _asartracked_qrcode))) (.Y (Math|Vector2D|BreakVector2D (Class|ARTrackedImage|GetEstimateSize _asartracked_qrcode)))) 2.0) "(R=0.000000,G=0.207111,B=1.000000,A=1.000000)" (Math|Transform|TransformRotation (Class|ARTrackedGeometry|GetLocaltoWorldTransform _asartracked_qrcode) "-90.000000, 0,0.000000") 0.0 0.0)
        (elif (Class|QRItemDictionary|KeyExists _qritemdict (Variables|/Script/AugmentedReality.ARTrackedQRCode|GetQRCode _asartracked_qrcode)) ; Exists
          (Rendering|Debug|DrawDebugBox (Math|Transform|TransformLocation (Class|ARTrackedGeometry|GetLocaltoWorldTransform _asartracked_qrcode) (/ (Math|Vector|MakeVector 0.3 (.X (Math|Vector2D|BreakVector2D (Class|ARTrackedImage|GetEstimateSize _asartracked_qrcode))) (.Y (Math|Vector2D|BreakVector2D (Class|ARTrackedImage|GetEstimateSize _asartracked_qrcode)))) 2.0)) (/ (Math|Vector|MakeVector 0.3 (.X (Math|Vector2D|BreakVector2D (Class|ARTrackedImage|GetEstimateSize _asartracked_qrcode))) (.Y (Math|Vector2D|BreakVector2D (Class|ARTrackedImage|GetEstimateSize _asartracked_qrcode)))) 2.0) "(R=0.021389,G=1.000000,B=0.000000,A=1.000000)" (Math|Transform|TransformRotation (Class|ARTrackedGeometry|GetLocaltoWorldTransform _asartracked_qrcode) "-90.000000, 0,0.000000") 0.0 0.0)
          (if (Variables|Default|GetSemaforo)
            (Development|PrintString "Semaforo ROJO" false false "(R=1.000000,G=0.015526,B=0.000000,A=1.000000)")
            (else
              (Variables|Default|SetSemaforo true)
              (Development|PrintString (Utilities|String|ToString(Rotator) (Math|Transform|TransformRotation (Class|ARTrackedGeometry|GetLocaltoWorldTransform _asartracked_qrcode) "-90.000000, 0,0.000000")) false false)
              (Class|QRItemDictionary|SpawnQRItems _qritemdict (Variables|/Script/AugmentedReality.ARTrackedQRCode|GetQRCode _asartracked_qrcode) (Math|Transform|TransformLocation (Class|ARTrackedGeometry|GetLocaltoWorldTransform _asartracked_qrcode) (/ (Math|Vector|MakeVector 0.3 (.X (Math|Vector2D|BreakVector2D (Class|ARTrackedImage|GetEstimateSize _asartracked_qrcode))) (.Y (Math|Vector2D|BreakVector2D (Class|ARTrackedImage|GetEstimateSize _asartracked_qrcode)))) 2.0)) (Math|Transform|TransformRotation (Class|ARTrackedGeometry|GetLocaltoWorldTransform _asartracked_qrcode) "-90.000000, 0,0.000000") (/ (Math|Vector|MakeVector 0.3 (.X (Math|Vector2D|BreakVector2D (Class|ARTrackedImage|GetEstimateSize _asartracked_qrcode))) (.Y (Math|Vector2D|BreakVector2D (Class|ARTrackedImage|GetEstimateSize _asartracked_qrcode)))) 2.0))
              (Utilities|Set|Add _spawedqrs (Variables|/Script/AugmentedReality.ARTrackedQRCode|GetQRCode _asartracked_qrcode))
              (Variables|Default|SetSemaforo false)))
          (else
            (Rendering|Debug|DrawDebugBox (Math|Transform|TransformLocation (Class|ARTrackedGeometry|GetLocaltoWorldTransform _asartracked_qrcode) (/ (Math|Vector|MakeVector 0.3 (.X (Math|Vector2D|BreakVector2D (Class|ARTrackedImage|GetEstimateSize _asartracked_qrcode))) (.Y (Math|Vector2D|BreakVector2D (Class|ARTrackedImage|GetEstimateSize _asartracked_qrcode)))) 2.0)) (/ (Math|Vector|MakeVector 0.3 (.X (Math|Vector2D|BreakVector2D (Class|ARTrackedImage|GetEstimateSize _asartracked_qrcode))) (.Y (Math|Vector2D|BreakVector2D (Class|ARTrackedImage|GetEstimateSize _asartracked_qrcode)))) 2.0) "(R=1.000000,G=0.000000,B=0.034335,A=1.000000)" (Math|Transform|TransformRotation (Class|ARTrackedGeometry|GetLocaltoWorldTransform _asartracked_qrcode) "-90.000000, 0,0.000000") 0.0 0.0)))))))

(event Custom|Degub)

(event Custom|OnTimerDelay
  (Class|ARBlueprintLibrary|ToggleARCapture true "QRCode"))

(event EventBeginPlay
  (Utilities|Time|SetTimerbyEvent (delegate Custom|OnTimerDelay) 5.0)
  (Utilities|Time|SetTimerbyEvent (delegate Custom|Degub) 3.0 true)
  (bind _returnvalue (Class|QRItemDictionary|CreateInstance (Utilities|String|Append (Class|KismetSystemLibrary|GetProjectContentDirectory) "JSONDicts/qr_objects.json")))
  (Variables|Default|SetQRItemDict _returnvalue))

(event EventEndPlay
  (params (EndPlayReason :type EEndPlayReason%20Enum :default "Destroyed"))
  (Class|ARBlueprintLibrary|ToggleARCapture false "QRCode"))

(fn ConstructionScript)