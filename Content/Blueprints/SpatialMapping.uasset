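; Spatial mapping Blueprint that switches on AR spatial mapping capture shortly after play begins and switches it off at end play.
; An ARTrackableNotify update event takes each tracked geometry's underlying mesh and, while the AR session is running, records it uniquely.
; It sets that mesh's material according to the SpatialMappingRenderMesh flag, using BaseMat when rendering is enabled.
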(event OnUpdateTrackedGeometry(ARTrackableNotify)
  (params (TrackedGeometry :type AR%20Tracked%20Geometry%20Object%20Reference))
  (bind _returnvalue (Class|ARBlueprintLibrary|GetARSessionStatus))
  (bind _returnvalue_2 (Class|ARTrackedGeometry|GetUnderlyingMesh TrackedGeometry))
  (bind (_additionalinfo _status) (Utilities|Struct|BreakARSessionStatus _returnvalue))
  (Utilities|IsValid _returnvalue_2
    (:Is%20Valid
      (if (Utilities|Enum|Equal(Enum) _status "Running")
        (Utilities|Array|AddUnique (Variables|Default|GetTracked%20Geometry) _returnvalue_2)
        (Rendering|Material|SetMaterial _returnvalue_2 0 (select (Variables|Default|GetSpatial%20Mapping%20Render%20Mesh) "/Game/BaseMat.BaseMat" 0))
        (else
          (Development|PrintString (Utilities|String|Append "ARSession ERROR:" (Utilities|String|EnumtoString _status) _additionalinfo) false false))))))

(event Custom|StartMapping
  (Class|ARBlueprintLibrary|ToggleARCapture true "SpatialMapping"))

(event EventBeginPlay
  (Utilities|Time|SetTimerbyEvent (delegate Custom|StartMapping) 4.0))

(event Collision|EventActorBeginOverlap
  (params (OtherActor :type Actor%20Object%20Reference)))

(event EventTick
  (params (DeltaSeconds :type Float%20%28single-precision%29)))

(event EventEndPlay
  (params (EndPlayReason :type EEndPlayReason%20Enum :default "Destroyed"))
  (Class|ARBlueprintLibrary|ToggleARCapture false "SpatialMapping"))

(fn ConstructionScript)