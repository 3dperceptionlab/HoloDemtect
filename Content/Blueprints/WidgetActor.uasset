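; WidgetActor is a world-space host for a UMG widget with a background, configured per XR device.
; The construction script detects the device type and, on Oculus HMD, destroys the UxtFollow and UxtWidget components and repositions Widget and Background at fixed relative offsets.
; SetWidget assigns the displayed widget and shows the whole component hierarchy, while SetVisibility toggles that hierarchy from the root.
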(event EventBeginPlay)

(event Collision|EventActorBeginOverlap
  (params (OtherActor :type Actor%20Object%20Reference)))

(event EventTick
  (params (DeltaSeconds :type Float%20%28single-precision%29)))

(fn ConstructionScript
  (bind _self self)
  (bind _devicetype (CallFunction|GetDeviceType))
  (bind _output_get (Variables|Default|SetDevice%20Type _devicetype))
  (switch Utilities|FlowControl|Switch|SwitchonDeviceType _output_get
    (:NewEnumerator1
      (Components|DestroyComponent (Variables|Default|GetUxtFollow _self))
      (Components|DestroyComponent (Variables|Default|GetUxtWidget _self))
      (Transformation|SetRelativeLocationAndRotation (Variables|Default|GetWidget) "27.000000, 0, 0" "0,180.000000, 0" false false)
      (Transformation|SetRelativeLocation (Variables|Default|GetBackground) "29.000000, 0, 0" false false))))

(fn SetWidget
  (params (Widget :type User%20Widget%20Object%20Reference))
  (UserInterface|SetWidget (Variables|Default|GetWidget) Widget)
  (Rendering|SetVisibility (Variables|Default|GetDefaultSceneRoot) true true))

(fn SetVisibility
  (params (Visible :type Boolean))
  (Rendering|SetVisibility (Variables|Default|GetDefaultSceneRoot) Visible true))