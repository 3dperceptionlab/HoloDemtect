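; WidgetHandMenu is a UX Tools (Uxt) hand menu actor with a pressable button and a text display, both held as child actors.
; On BeginPlay it binds the button press and subscribes to the MRPawn's HandMenuText event.
; A press fires the Button1HandMenuClicked dispatcher, while text broadcast by the pawn is written to the second child's UxtTextRenderActor.
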(event Custom|CustomEvent_0
  (params (Button :type Uxt%20Pressable%20Button%20Component%20Object%20Reference) (Pointer :type Uxt%20Pointer%20Component%20Object%20Reference))
  (Default|CallButton1HandMenuClicked))

(event Custom|UpdateText
  (params (Text :type String))
  (bind _asuxt_text_render_actor (Utilities|Casting|CastToUxtTextRenderActor (Variables|/Script/Engine.ChildActorComponent|GetChildActor (Variables|Default|GetButton_2))))
  (Rendering|Components|TextRender|SetText (Variables|/Script/UXTools.UxtTextRenderActor|GetTextRender _asuxt_text_render_actor) (Utilities|Text|ToText(String) Text)))

(event EventBeginPlay
  (EventDispatchers|BindEventtoOnButtonPressed (Actor|GetComponentbyClass (Variables|/Script/Engine.ChildActorComponent|GetChildActor (Variables|Default|GetButton_1)) "/Script/UXTools.UxtPressableButtonComponent") (delegate Custom|CustomEvent_0))
  (bind _asmrpawn (Utilities|Casting|CastToMRPawn (Game|Player|GetPlayerPawn 0)))
  (EventDispatchers|BindEventtoHandMenuText _asmrpawn (delegate Custom|UpdateText)))

(fn ConstructionScript
  (|CallParentFunction))